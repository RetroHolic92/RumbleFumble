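; BP_TraitorDetector is the traitor detector item Blueprint; the only logic here plays a drop sound when its StaticMesh hits something.
; The hit component's speed is remapped into the sound cue's integer "power" parameter and its volume multiplier.
; A DoOnce, reset after a short random delay, throttles the sound during repeated hits.
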(event `self.StaticMesh.OnComponentHit`
  (params (HitComponent :type "PrimitiveComponent Object Reference") (OtherActor :type "Actor Object Reference") (OtherComp :type "PrimitiveComponent Object Reference") (NormalImpulse :type "Vector Structure") (Hit :type "HitResult Structure (by ref)"))
  (bind _returnvalue (`KismetMathLibrary.VSize` (`SceneComponent.GetComponentVelocity` HitComponent)))
  (`|ExecutionSequence`
    (:`then_0`
      (`/Engine/EditorBlueprintResources/StandardMacros.DoOnce` false :!label _label
        (:`Completed`
          (bind _returnvalue_2 (`GameplayStatics.SpawnSoundAtLocation` "/Game/Assets/Sounds/Item_Drop_SoundCue.Item_Drop_SoundCue" Hit_Location (struct) 1.0 1.0 0.0 null null))
          (`AudioComponent.SetIntParameter` _returnvalue_2 "power" (`KismetMathLibrary.FTrunc` (`KismetMathLibrary.MapRangeClamped` _returnvalue 400.0 30.0 0.0 8.0)))
          (`AudioComponent.SetVolumeMultiplier` _returnvalue_2 (`KismetMathLibrary.MapRangeClamped` _returnvalue 30.0 0.0 1.0)))))
    (:`then_1`
      (`KismetSystemLibrary.Delay` (`KismetMathLibrary.RandomFloatInRange` 0.1 0.2))
      (goto _label :!via `Reset`))))

(fn `UserConstructionScript`)